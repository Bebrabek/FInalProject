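; BP_GameCharacter is a player character Blueprint that handles jumping and interaction with nearby objects.
; Enhanced Input actions drive Jump, StopJumping and interact.
; Capsule overlaps store the first actor implementing BPI_Interactable as CurrentInteract while none is held, and clear it when that actor leaves.
; The interact input sends InteractMessage to the stored actor if it is valid.
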(event `EnhancedInput|/Game/MyProject/Core/EnhancedInput/Action/IA_GameJump`
  (params (ActionValue :type "Vector2D Structure") (ElapsedSeconds :type "Float (double-precision)") (TriggeredSeconds :type "Float (double-precision)") (InputAction :type "InputAction Object Reference" :default "/Game/MyProject/Core/EnhancedInput/Action/IA_GameJump.IA_GameJump"))
  (:`Triggered`
    (`self.Jump`))
  (:`Completed`
    (`self.StopJumping`)))

(event `self.CapsuleComponent.OnComponentBeginOverlap`
  (params (OverlappedComponent :type "PrimitiveComponent Object Reference") (OtherActor :type "Actor Object Reference") (OtherComp :type "PrimitiveComponent Object Reference") (OtherBodyIndex :type Integer) (bFromSweep :type Boolean) (SweepResult :type "HitResult Structure (by ref)"))
  (if (`KismetSystemLibrary.DoesImplementInterface` OtherActor "/Game/MyProject/Core/BPI/BPI_Interactable.BPI_Interactable_C")
    (`/Engine/EditorBlueprintResources/StandardMacros.IsValid` (`self.CurrentInteract`)
      (:`Is Not Valid`
        (set `self.CurrentInteract` OtherActor)))))

(event `self.CapsuleComponent.OnComponentEndOverlap`
  (params (OverlappedComponent :type "PrimitiveComponent Object Reference") (OtherActor :type "Actor Object Reference") (OtherComp :type "PrimitiveComponent Object Reference") (OtherBodyIndex :type Integer))
  (if (== OtherActor (`self.CurrentInteract`))
    (set `self.CurrentInteract` null)))

(event `EnhancedInput|/Game/MyProject/Core/EnhancedInput/Action/IA_Interact`
  (params (ActionValue :type Boolean) (ElapsedSeconds :type "Float (double-precision)") (TriggeredSeconds :type "Float (double-precision)") (InputAction :type "InputAction Object Reference" :default "/Game/MyProject/Core/EnhancedInput/Action/IA_Interact.IA_Interact"))
  (bind _currentinteract (`self.CurrentInteract`))
  (:`Triggered`
    (`/Engine/EditorBlueprintResources/StandardMacros.IsValid` _currentinteract
      (:`Is Valid`
        (message `/Game/MyProject/Core/BPI/BPI_Interactable.Interact` _currentinteract)))))

(fn `UserConstructionScript`)