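; BP_WinCollision is an overlap actor that ends play and shows the game-over screen.
; Any actor overlap triggers it, as it only casts player 0's character to BP_GameCharacter without checking the overlapping actor.
; It destroys that character, removes PlayerInterface if valid, then adds WBP_GameOverScreen to the viewport with UI-only input and a visible cursor.
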(event `self.ReceiveActorBeginOverlap`
  (params (OtherActor :type "Actor Object Reference"))
  (bind _returnvalue (`GameplayStatics.GetPlayerController` 0))
  (bind _asbp_game_character (cast `/Game/MyProject/Character/BP_GameCharacter` (`GameplayStatics.GetPlayerCharacter` 0)))
  (`self.K2_DestroyActor` _asbp_game_character)
  (`|ExecutionSequence`
    (:`then_0`
      (bind _playerinterface (`self.PlayerInterface`)
        (:`then`
          (`Widget.RemoveFromParent` _playerinterface))
        (:`else`)))
    (:`then_1`
      (bind _returnvalue_2 (`|CreateWidget` "/Game/MyProject/UI/WBP_GameOverScreen.WBP_GameOverScreen_C" _returnvalue))
      (`UserWidget.AddToViewport` _returnvalue_2 0)
      (`WidgetBlueprintLibrary.SetInputMode_UIOnlyEx` _returnvalue _returnvalue_2)
      (set `PlayerController.bShowMouseCursor` true _returnvalue))))

(fn `UserConstructionScript`)