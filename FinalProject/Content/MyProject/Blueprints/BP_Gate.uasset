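; BP_Gate is a gate that slides its Cube mesh vertically, with events to open and close it.
; OpenGate plays a timeline that drives the cube's relative Z up to 300 units, and CloseGate reverses it.
; On BeginPlay it binds to the OnPressed dispatcher of a single BP_ButtonGate and to the CloseGate dispatcher of all BP_Camera actors.
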(event `OpenGate`
  (bind (_direction _gatetrack) (`Timeline|GateTimeline` :`NewTime` 0.0 :!label _label)
    (:`Update`
      (`SceneComponent.K2_SetRelativeLocation` (`self.Cube`) (`KismetMathLibrary.MakeVector` 0.0 0.0 (* _gatetrack 300.0)) false false))))

(event `CloseGate`
  (goto _label :!via `Reverse`))

(event `self.ReceiveBeginPlay`
  (`|ExecutionSequence`
    (:`then_0`
      (bind _returnvalue (`GameplayStatics.GetActorOfClass` "/Game/MyProject/Blueprints/BP_ButtonGate.BP_ButtonGate_C"))
      (add `/Game/MyProject/Blueprints/BP_ButtonGate.OnPressed` _returnvalue (`|CreateDelegate` :!event `OpenGate`)))
    (:`then_1`
      (bind _outactors (`GameplayStatics.GetAllActorsOfClass` "/Game/MyProject/Blueprints/Pawns/BP_Camera.BP_Camera_C"))
      (add `/Game/MyProject/Blueprints/Pawns/BP_Camera.CloseGate` _outactors (`|CreateDelegate` :!event `CloseGate`)))))

(fn `UserConstructionScript`)