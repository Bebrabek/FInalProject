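; BP_PointLight is an interactable point light actor that also signals switchable actors in the level.
; On Interact, it toggles the PointLight component's visibility, then loops over every BPI_Switchable actor.
; Each one receives SwitchOn if it reports being on, otherwise SwitchOff, through interface messages.
; Its IsSwitchOn function returns the IsOn variable, which this graph never updates.
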(event `/Game/MyProject/Core/BPI/BPI_Interactable.Interact`
  (`SceneComponent.ToggleVisibility` (`self.PointLight`) false)
  (bind _outactors (`GameplayStatics.GetAllActorsWithInterface` "/Game/MyProject/Core/BPI/BPI_Switchable.BPI_Switchable_C"))
  (for _array_element _outactors
    (bind _ison (message `/Game/MyProject/Core/BPI/BPI_Switchable.IsSwitchOn` _array_element))
    (if _ison
      (message `/Game/MyProject/Core/BPI/BPI_Switchable.SwitchOn` _array_element)
      (else
        (message `/Game/MyProject/Core/BPI/BPI_Switchable.SwitchOff` _array_element)))))

(fn `IsSwitchOn`
  (returns (IsOn :type Boolean))
  (return (`self.IsOn`)))

(fn `UserConstructionScript`
  (`parent.UserConstructionScript`))