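; BP_Camera is a security camera that sweeps back and forth and signals a gate to close when it spots the player.
; A looping timeline lerps the skeletal mesh between its starting rotation and a 180-degree yaw offset, swapping direction on each finish.
; Tick runs a Patrol/Find state machine: a forward sphere trace detects BP_GameCharacter, then Find calls CloseGate and returns to Patrol.
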(event `self.ReceiveBeginPlay`
  (bind _output_get (set `self.StartRotation` (`SceneComponent.K2_GetComponentRotation` (`self.SkeletalMesh`))))
  (set `self.EndRotation` (`KismetMathLibrary.MakeRotator` (.roll _output_get) (.pitch _output_get) (+ (.yaw _output_get) 180.0)))
  (set `self.CurrentRotation` (`self.StartRotation`))
  (set `self.TargretRotation` (`self.EndRotation`))
  (`self.StartPatrol`))

(event `StartPatrol`
  (bind (_direction _rotatetrack) (`Timeline|Шкала времени` :!via `PlayFromStart`)
    (:`Update`
      (`SceneComponent.K2_SetWorldRotation` (`self.SkeletalMesh`) (`KismetMathLibrary.RLerp` (`self.CurrentRotation`) (`self.TargretRotation`) _rotatetrack) false false))
    (:`Finished`
      (switch `ETimelineDirection` (`self.DirectionMove`)
        (:`Forward`
          (set `self.DirectionMove` "Backward")
          (set `self.TargretRotation` (`self.StartRotation`))
          (set `self.CurrentRotation` (`self.EndRotation`)))
        (:`Backward`
          (set `self.DirectionMove` "Forward")
          (set `self.CurrentRotation` (`self.StartRotation`))
          (set `self.TargretRotation` (`self.EndRotation`))))
      (`self.StartPatrol`))))

(event `self.ReceiveTick`
  (params (DeltaSeconds :type "Float (single-precision)"))
  (switch `/Game/MyProject/Core/Enum/E_Camera` (`self.CurrentState`)
    (:`NewEnumerator0`
      (bind _isplayerfind (`self.PlayerSearch`))
      (if _isplayerfind
        (set `self.CurrentState` "NewEnumerator1")))
    (:`NewEnumerator1`
      (`self.CloseGate`)
      (`self.PlayerSearch`)
      (set `self.CurrentState` "NewEnumerator0"))))

(fn `PlayerSearch`
  (returns (IsPlayerFind :type Boolean))
  (bind _scene (`self.Scene`))
  (bind _returnvalue (`SceneComponent.K2_GetComponentLocation` _scene))
  (bind (_outhit _returnvalue_2) (`KismetSystemLibrary.SphereTraceSingle` _returnvalue (+ _returnvalue (* (`SceneComponent.GetForwardVector` _scene) (`self.SearchDistance`))) 100.0 "TraceTypeQuery3"))
  (if _returnvalue_2
    (cast `/Game/MyProject/Character/BP_GameCharacter` (`.HitActor` (`GameplayStatics.BreakHitResult` _outhit))
      (:`then`
        (return true))
      (:`CastFailed`
        (return false)))
    (else
      (return false))))

(fn `UserConstructionScript`)