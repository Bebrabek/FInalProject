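; BP_GamePlayerController is the in-game player controller that turns Enhanced Input into character movement and camera look.
; On BeginPlay it sets game-only input, hides the cursor, adds the IMC_Game mapping context and caches the controlled BP_GameCharacter's movement component.
; Move input feeds that component directly along control-rotation-relative forward and right vectors, ignoring pitch.
; Look input drives controller yaw and pitch.
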(event `self.ReceiveBeginPlay`
  (`WidgetBlueprintLibrary.SetInputMode_GameOnly` self)
  (set `self.bShowMouseCursor` false)
  (`EnhancedInputSubsystemInterface.AddMappingContext` (subsystem `EnhancedInputLocalPlayerSubsystem`) "/Game/MyProject/Core/EnhancedInput/IMC_Game.IMC_Game" 0 (struct))
  (bind _asbp_game_character (cast `/Game/MyProject/Character/BP_GameCharacter` (`self.K2_GetPawn`)))
  (bind _output_get (set `self.As BP Game Character` _asbp_game_character))
  (set `self.CharacterMovement` (`Character.CharacterMovement` _output_get)))

(event `EnhancedInput|/Game/MyProject/Core/EnhancedInput/Action/IA_GameMove`
  (params (ActionValue :type "Vector2D Structure") (ElapsedSeconds :type "Float (double-precision)") (TriggeredSeconds :type "Float (double-precision)") (InputAction :type "InputAction Object Reference" :default "/Game/MyProject/Core/EnhancedInput/Action/IA_GameMove.IA_GameMove"))
  (bind (_returnvalue_roll _returnvalue_pitch _returnvalue_yaw) (`KismetMathLibrary.BreakRotator` (`self.GetControlRotation`)))
  (bind (_returnvalue_roll_2 _returnvalue_pitch_2 _returnvalue_yaw_2) (`KismetMathLibrary.BreakRotator` (`self.GetControlRotation`)))
  (:`Triggered`
    (bind _charactermovement (`self.CharacterMovement`)
      (:`then`
        (`|ExecutionSequence`
          (:`then_0`
            (`PawnMovementComponent.AddInputVector` _charactermovement (* (`KismetMathLibrary.GetForwardVector` (`KismetMathLibrary.MakeRotator` 0.0 0.0 _returnvalue_yaw)) ActionValue_Y) false))
          (:`then_1`
            (`PawnMovementComponent.AddInputVector` _charactermovement (* (`KismetMathLibrary.GetRightVector` (`KismetMathLibrary.MakeRotator` _returnvalue_roll_2 0.0 _returnvalue_yaw_2)) ActionValue_X) false))))
      (:`else`))))

(event `EnhancedInput|/Game/MyProject/Core/EnhancedInput/Action/IA_GameLook`
  (params (ActionValue :type "Vector2D Structure") (ElapsedSeconds :type "Float (double-precision)") (TriggeredSeconds :type "Float (double-precision)") (InputAction :type "InputAction Object Reference" :default "/Game/MyProject/Core/EnhancedInput/Action/IA_GameLook.IA_GameLook"))
  (:`Triggered`
    (`self.AddYawInput` ActionValue_X)
    (`self.AddPitchInput` ActionValue_Y)))

(fn `UserConstructionScript`)